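; Cart Blueprint actor that animates a hammer swinging back and forth along a spline, starting on BeginPlay.
; A looping ping-pong timeline drives the hammer mesh's position by spline distance up to the second point.
; The same curve samples spline rotation, remapping pitch to roll and offsetting yaw to orient the hammer.
; Tick draws a debug sphere at the spline's start.
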(event `self.ReceiveBeginPlay`
  (bind _hammerswingspline (`self.HammerSwingSpline`))
  (bind (_direction _outcurve) (`Timeline|HammerSwingtimeline` :!label _label)
    (:`Update`
      (`SceneComponent.K2_SetWorldLocation` (`self.HammerMesh`) (`SplineComponent.GetLocationAtDistanceAlongSpline` (`self.HammerSwingSpline`) (* (`SplineComponent.GetDistanceAlongSplineAtSplinePoint` _hammerswingspline 1) _outcurve) "World") false false)
      (bind (_returnvalue_roll _returnvalue_pitch _returnvalue_yaw) (`KismetMathLibrary.BreakRotator` (`SplineComponent.GetRotationAtTime` _hammerswingspline _outcurve "Local" false)))
      (`SceneComponent.K2_SetRelativeRotation` (`self.HammerMesh`) (`KismetMathLibrary.MakeRotator` _returnvalue_pitch 0.0 (+ _returnvalue_yaw 90.0)) false false))
    (:`Finished`
      (if (`|EnumEquality` _direction "Forward")
        (goto _label :!via `ReverseFromEnd`)
        (else
          (goto _label))))))

(event `self.ReceiveTick`
  (params (DeltaSeconds :type "Float (single-precision)"))
  (`KismetSystemLibrary.DrawDebugSphere` (`SplineComponent.GetLocationAtDistanceAlongSpline` (`self.HammerSwingSpline`) 0.0 "World") 2.0 12 (struct :`R` 1.0 :`G` 0.03409 :`A` 1.0) 0.1))

(fn `UserConstructionScript`)