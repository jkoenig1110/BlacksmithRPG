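; Anvil actor that hosts a forging minigame, showing the ForgeMinigame widget and mouse cursor when the player overlaps it.
; DropHammerAnim plays a timeline from a given start position, moving the hammer along a spline at a rate scaled by that position.
; On finish it plays a hit sound and sparks, then opens a Tick-fed gate that eases the hammer back to HammeringScene until the next drop.
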(event `self.ReceiveActorBeginOverlap`
  (params (OtherActor :type "Actor Object Reference"))
  (bind _asplayer_bp (cast `/Game/Blueprints/Player/PlayerBP` OtherActor))
  (bind _ascontroller_bp (cast `/Game/Blueprints/Player/ControllerBP` (`Pawn.GetController` _asplayer_bp)))
  (`WidgetBlueprintLibrary.SetInputMode_GameAndUIEx` _ascontroller_bp (`self.GameWidget`))
  (set `PlayerController.bShowMouseCursor` true _ascontroller_bp)
  (`UserWidget.AddToViewport` (`self.GameWidget`) 0)
  (`TimelineComponent.SetPlayRate` (`self.HammerDropTimeline`) (`self.BasePlayRate`)))

(event `self.ReceiveActorEndOverlap`
  (params (OtherActor :type "Actor Object Reference"))
  (if (== OtherActor (`GameplayStatics.GetPlayerCharacter` 0))
    (`Widget.RemoveFromParent` (`self.GameWidget`))))

(event `self.ReceiveBeginPlay`
  (bind _returnvalue (`|CreateWidget` "/Game/Blueprints/Minigame/ForgeMinigame.ForgeMinigame_C" null self))
  (set `self.GameWidget` _returnvalue))

(event `DropHammerAnim`
  (params (InStartPosition :type "Float (double-precision)"))
  (bind _baseplayrate (`self.BasePlayRate`))
  (bind _hammermesh (`self.HammerMesh`))
  (bind _hammeringscene (`self.HammeringScene`))
  (bind _hammerswingspline (`self.HammerSwingSpline`))
  (bind _hammermesh_2 (`self.HammerMesh`))
  (bind _returnvalue (`SceneComponent.K2_GetComponentLocation` _hammermesh))
  (`|ExecutionSequence`
    (:`then_0`
      (`TimelineComponent.SetPlayRate` (`self.HammerDropTimeline`) (`KismetMathLibrary.FClamp` (* _baseplayrate (- 1.0 InStartPosition)) 1.0 _baseplayrate))
      (`|ExecutionSequence`
        (:`then_0`
          (bind (_direction _swingcurve) (`Timeline|HammerDropTimeline` :`NewTime` InStartPosition :!via `SetNewTime` :!label _label)
            (:`Update`
              (`SceneComponent.K2_SetWorldLocationAndRotation` _hammermesh (`SplineComponent.GetLocationAtTime` _hammerswingspline _swingcurve "World" false) (`SplineComponent.GetRotationAtTime` _hammerswingspline _swingcurve "World" false) false false))
            (:`Finished`
              (`GameplayStatics.PlaySoundAtLocation` "/Game/Audio/Sounds/CleanHitCue.CleanHitCue" _returnvalue (struct) 1.0 1.0 0.0 null null null)
              (`GameplayStatics.SpawnEmitterAtLocation` "/Game/Particles/ForgeHammerSparks.ForgeHammerSparks" _returnvalue)
              (goto _label_2 :!via `Open`))))
        (:`then_1`
          (goto _label_2 :!via `Close`))))
    (:`then_1`
      (goto _label))))

(event `self.ReceiveTick`
  (params (DeltaSeconds :type "Float (single-precision)"))
  (bind _hammeringscene (`self.HammeringScene`))
  (bind _hammermesh (`self.HammerMesh`))
  (`/Engine/EditorBlueprintResources/StandardMacros.Gate` true :!label _label_2
    (:`Exit`
      (`SceneComponent.K2_SetWorldLocationAndRotation` (`self.HammerMesh`) (`KismetMathLibrary.VInterpTo` (`SceneComponent.K2_GetComponentLocation` _hammermesh) (`SceneComponent.K2_GetComponentLocation` _hammeringscene) DeltaSeconds 2.0) (`KismetMathLibrary.RInterpTo` (`SceneComponent.K2_GetComponentRotation` _hammermesh) (`SceneComponent.K2_GetComponentRotation` _hammeringscene) DeltaSeconds 2.0) false false))))

(fn `UserConstructionScript`)