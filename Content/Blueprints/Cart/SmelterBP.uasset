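; Smelter actor that lets the player turn Copper, Tin or Iron ore from their inventory into ingots.
; On player overlap it shows the SmelterPrompt widget with a mouse cursor and totals each ore type, removing the prompt on exit.
; MakeIngot swaps one ore for one ingot of the chosen metal and refreshes the totals.
; Ore and ingot items are constructed from data table rows keyed by metal name.
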(event `self.ReceiveBeginPlay`
  (bind _returnvalue (`|CreateWidget` "/Game/Blueprints/Minigame/SmelterPrompt.SmelterPrompt_C" null self))
  (set `self.SmelterWidget` _returnvalue))

(event `self.ReceiveActorBeginOverlap`
  (params (OtherActor :type "Actor Object Reference"))
  (bind _playerinventory (`/Game/Blueprints/Player/ControllerBP.PlayerInventory` (`self.PlayerController`)))
  (bind _asplayer_bp (cast `/Game/Blueprints/Player/PlayerBP` OtherActor))
  (bind _ascontroller_bp (cast `/Game/Blueprints/Player/ControllerBP` (`Pawn.GetController` _asplayer_bp)))
  (bind _output_get (set `self.PlayerController` _ascontroller_bp))
  (`WidgetBlueprintLibrary.SetInputMode_GameAndUIEx` _ascontroller_bp (`self.SmelterWidget`))
  (set `PlayerController.bShowMouseCursor` true _ascontroller_bp)
  (`UserWidget.AddToViewport` (`self.SmelterWidget`) 0)
  (bind _outitem (`self.ConstructOre` "Copper"))
  (bind _outitem_2 (`self.ConstructOre` "Tin"))
  (bind _outitem_3 (`self.ConstructOre` "Iron"))
  (set `self.CopperTotal` 0 :!label _label)
  (set `self.TinTotal` 0)
  (set `self.IronTotal` 0)
  (for _array_element (`/Game/Blueprints/Inventory/InventoryManager.InventoryArray` _playerinventory)
    (bind _itemsaresame (`/Game/Blueprints/Inventory/InventoryManager.CompareItems` _playerinventory _outitem _array_element))
    (if _itemsaresame
      (bind _amountinstack (`/Game/Blueprints/Inventory/ItemObject/Item_Generic.AmountInStack` _array_element))
      (set `self.CopperTotal` (+ (`self.CopperTotal`) _amountinstack))
      (else
        (bind _itemsaresame_2 (`/Game/Blueprints/Inventory/InventoryManager.CompareItems` _playerinventory _outitem_2 _array_element))
        (if _itemsaresame_2
          (set `self.TinTotal` (+ (`self.TinTotal`) _amountinstack))
          (else
            (bind _itemsaresame_3 (`/Game/Blueprints/Inventory/InventoryManager.CompareItems` _playerinventory _outitem_3 _array_element))
            (if _itemsaresame_3
              (set `self.IronTotal` (+ (`self.IronTotal`) _amountinstack)))))))))

(event `self.ReceiveActorEndOverlap`
  (params (OtherActor :type "Actor Object Reference"))
  (bind _smelterwidget (`self.SmelterWidget`))
  (if (== OtherActor (`GameplayStatics.GetPlayerCharacter` 0))
    (`Widget.RemoveFromParent` _smelterwidget)
    (`Widget.RemoveFromParent` _smelterwidget)
    (`WidgetBlueprintLibrary.SetInputMode_GameOnly` (stale `self.ReceiveActorBeginOverlap` _output_get))
    (set `PlayerController.bShowMouseCursor` false (stale `self.ReceiveActorBeginOverlap` _output_get))))

(event `MakeIngot`
  (params (InMetalType :type "/Game/Blueprints/Inventory/Data/EMaterial Enum" :default "NewEnumerator0"))
  (bind _playerinventory (`/Game/Blueprints/Player/ControllerBP.PlayerInventory` (`self.PlayerController`)))
  (bind _inventoryarray (`/Game/Blueprints/Inventory/InventoryManager.InventoryArray` _playerinventory))
  (switch `/Game/Blueprints/Inventory/Data/EMaterial` InMetalType
    (:`NewEnumerator0`
      (if (> (`self.CopperTotal`) 0)
        (bind _outitem (`self.ConstructIngot` "Copper"))
        (set `self.IngotItemToAdd` _outitem)
        (bind _outitem_2 (`self.ConstructOre` "Copper"))
        (set `self.CompareSmeltOre` _outitem_2)
        (for (_array_element _array_index) _inventoryarray :!label _label_2
          (bind _itemsaresame (`/Game/Blueprints/Inventory/InventoryManager.CompareItems` _playerinventory (`self.CompareSmeltOre`) _array_element))
          (if _itemsaresame
            (bind _output_get (set `self.InventoryReplaceItem` (`|GetArrayItem` _inventoryarray _array_index)))
            (bind _amountinstack (`/Game/Blueprints/Inventory/ItemObject/Item_Generic.AmountInStack` _output_get))
            (`/Engine/EditorBlueprintResources/StandardMacros.DecrementInt` _amountinstack
              (:`  `
                (if (<= _amountinstack 0)
                  (`/Game/Blueprints/Inventory/InventoryManager.ClearItemAtIndex` _playerinventory _array_index)
                  (else
                    (`KismetArrayLibrary.Array_Set` _inventoryarray _array_index (`self.InventoryReplaceItem`))))
                (`/Game/Blueprints/Inventory/InventoryManager.UpdateSlot` _playerinventory _array_index)
                (`/Game/Blueprints/Inventory/InventoryManager.AddItem` _playerinventory (`self.IngotItemToAdd`))
                (break)))))
        (goto _label)))
    (:`NewEnumerator1`
      (if (> (`self.TinTotal`) 0)
        (bind _outitem_3 (`self.ConstructIngot` "Tin"))
        (set `self.IngotItemToAdd` _outitem_3)
        (bind _outitem_4 (`self.ConstructOre` "Tin"))
        (set `self.CompareSmeltOre` _outitem_4)
        (goto _label_2)))
    (:`NewEnumerator2`
      (if (> (`self.IronTotal`) 0)
        (bind _outitem_5 (`self.ConstructIngot` "Iron"))
        (set `self.IngotItemToAdd` _outitem_5)
        (bind _outitem_6 (`self.ConstructOre` "Iron"))
        (set `self.CompareSmeltOre` _outitem_6)
        (goto _label_2)))))

(fn `ConstructIngot`
  (params (InOreName :type String))
  (returns (OutItem :type "/Game/Blueprints/Inventory/ItemObject/Item_Generic Object Reference"))
  (bind _returnvalue (`|GetDataTableRow` "/Game/Blueprints/Inventory/Data/IngotTable.IngotTable" (`KismetStringLibrary.Conv_StringToName` (`KismetStringLibrary.Concat_StrStr` "Ingot_" InOreName)))
    (:`then`
      (bind _returnvalue_2 (`|GenericCreateObject` "/Game/Blueprints/Inventory/ItemObject/Item_Ingot.Item_Ingot_C" self null))
      (`/Game/Blueprints/Inventory/ItemObject/Item_Generic.Constructor` :`self` _returnvalue_2 :`InIngotStruct` _returnvalue)
      (`/Game/Blueprints/Inventory/ItemObject/Item_Generic.SetAmountInStack` _returnvalue_2 1)
      (return _returnvalue_2))))

(fn `ConstructOre`
  (params (InOreName :type String))
  (returns (OutItem :type "/Game/Blueprints/Inventory/ItemObject/Item_Generic Object Reference"))
  (bind _returnvalue (`|GetDataTableRow` "/Game/Blueprints/Inventory/Data/OreTable.OreTable" (`KismetStringLibrary.Conv_StringToName` (`KismetStringLibrary.Concat_StrStr` "Ore_" InOreName)))
    (:`then`
      (bind _returnvalue_2 (`|GenericCreateObject` "/Game/Blueprints/Inventory/ItemObject/Item_Ore.Item_Ore_C" self null))
      (`/Game/Blueprints/Inventory/ItemObject/Item_Generic.Constructor` :`self` _returnvalue_2 :`InOreStruct` _returnvalue)
      (return _returnvalue_2))))

(fn `UserConstructionScript`)