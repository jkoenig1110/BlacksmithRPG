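; World pickup actor for ore, ingot and weapon part items that offers its item to the player's inventory on overlap.
; On BeginPlay it uses its assigned Item, or rolls a random category, material or part name and stack amount.
; The rolled name keys a data table row that builds the item object, which supplies the mesh.
; The actor destroys itself when AddItem returns false or empty.
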(event `self.ReceiveBeginPlay`
  (bind _item (`self.Item`))
  (bind _dataname (`self.DataName`))
  (bind _returnvalue (`KismetStringLibrary.Conv_NameToString` (`self.DataName`)))
  (`/Engine/EditorBlueprintResources/StandardMacros.IsValid` _item
    (:`Is Valid`
      (set `self.Amount` (`/Game/Blueprints/Inventory/ItemObject/Item_Generic.AmountInStack` _item)))
    (:`Is Not Valid`
      (set `self.Amount` (`KismetMathLibrary.RandomIntegerInRange` 1 99))
      (set `self.ItemCat` (cast `/Game/Blueprints/Inventory/Data/EItemCat` (`KismetMathLibrary.Conv_IntToByte` (`KismetMathLibrary.RandomIntegerInRange` 1 3))))
      (set `self.ItemMaterial` (cast `/Game/Blueprints/Inventory/Data/EMaterial` (`KismetMathLibrary.Conv_IntToByte` (`KismetMathLibrary.RandomIntegerInRange` 0 2))))
      (switch `/Game/Blueprints/Inventory/Data/EItemCat` (`self.ItemCat`)
        (:`NewEnumerator0`
          (set `self.DataName` (`KismetStringLibrary.Conv_StringToName` (`KismetStringLibrary.Concat_StrStr` "" "Ore_")))
          (switch `/Game/Blueprints/Inventory/Data/EMaterial` (`self.ItemMaterial`) :!label _label
            (:`NewEnumerator0`
              (set `self.DataName` (`KismetStringLibrary.Conv_StringToName` (`KismetStringLibrary.Concat_StrStr` _returnvalue "Copper"))))
            (:`NewEnumerator1`
              (set `self.DataName` (`KismetStringLibrary.Conv_StringToName` (`KismetStringLibrary.Concat_StrStr` _returnvalue "Tin"))))
            (:`NewEnumerator2`
              (set `self.DataName` (`KismetStringLibrary.Conv_StringToName` (`KismetStringLibrary.Concat_StrStr` _returnvalue "Iron"))))))
        (:`NewEnumerator1`
          (set `self.DataName` (`KismetStringLibrary.Conv_StringToName` (`KismetStringLibrary.Concat_StrStr` "" "Ingot_")))
          (goto _label))
        (:`NewEnumerator2`
          (bind _newparam (`self.RandomPart`))
          (set `self.DataName` (`KismetStringLibrary.Conv_StringToName` _newparam))))
      (switch `/Game/Blueprints/Inventory/Data/EItemCat` (`self.ItemCat`)
        (:`NewEnumerator0`
          (bind _returnvalue_2 (`|GetDataTableRow` "/Game/Blueprints/Inventory/Data/OreTable.OreTable" _dataname)
            (:`then`
              (bind _returnvalue_3 (`|GenericCreateObject` "/Game/Blueprints/Inventory/ItemObject/Item_Ore.Item_Ore_C" self null))
              (`/Game/Blueprints/Inventory/ItemObject/Item_Generic.Constructor` :`self` _returnvalue_3 :`InOreStruct` _returnvalue_2)
              (set `self.Item` _returnvalue_3))))
        (:`NewEnumerator1`
          (bind _returnvalue_4 (`|GetDataTableRow` "/Game/Blueprints/Inventory/Data/IngotTable.IngotTable" _dataname)
            (:`then`
              (bind _returnvalue_5 (`|GenericCreateObject` "/Game/Blueprints/Inventory/ItemObject/Item_Ingot.Item_Ingot_C" self null))
              (`/Game/Blueprints/Inventory/ItemObject/Item_Generic.Constructor` :`self` _returnvalue_5 :`InIngotStruct` _returnvalue_4)
              (set `self.Item` _returnvalue_5))))
        (:`NewEnumerator2`
          (bind _returnvalue_6 (`|GetDataTableRow` "/Game/Blueprints/Inventory/Data/PartTable.PartTable" _dataname)
            (:`then`
              (bind _returnvalue_7 (`|GenericCreateObject` "/Game/Blueprints/Inventory/ItemObject/Item_Part.Item_Part_C" self null))
              (`/Game/Blueprints/Inventory/ItemObject/Item_Generic.Constructor` :`self` _returnvalue_7 :`InPartStruct` _returnvalue_6)
              (set `self.Item` _returnvalue_7)))))))
  (`StaticMeshComponent.SetStaticMesh` (`self.StaticMesh`) (`/Game/Blueprints/Inventory/ItemObject/Item_Generic.BaseMesh` (`self.Item`)))
  (`/Game/Blueprints/Inventory/ItemObject/Item_Generic.SetAmountInStack` (`self.Item`) (`self.Amount`)))

(event `self.ReceiveActorBeginOverlap`
  (params (OtherActor :type "Actor Object Reference"))
  (bind _asplayer_bp (cast `/Game/Blueprints/Player/PlayerBP` OtherActor))
  (bind _distributionfail (`/Game/Blueprints/Inventory/InventoryManager.AddItem` (`/Game/Blueprints/Player/ControllerBP.PlayerInventory` (cast `/Game/Blueprints/Player/ControllerBP` (`Pawn.GetController` _asplayer_bp) :!pure true)) (`self.Item`)))
  (if (not _distributionfail)
    (`self.K2_DestroyActor`)))

(fn `RandomPart`
  (returns (NewParam :type String))
  (locals (Rand :type Integer :default 0))
  (bind _returnvalue (`KismetMathLibrary.RandomIntegerInRange` 0 2))
  (bind _output_get (set `local.Rand` _returnvalue))
  (return (`KismetStringLibrary.Concat_StrStr` "Part_" (select `int` _output_get :`0` (select `int` _returnvalue :`0` "Sword" :`1` "Hammer" :`2` "Axe") :`1` (select `int` _returnvalue :`0` "Short" :`1` "Long" :`2` "Pole") :`2` (select `int` _returnvalue :`0` "Crossguard" :`1` "Pommel" :`2` "Spike")) (select `int` _output_get :`0` "Head" :`1` "Handle" :`2` "Extra"))))

(fn `UserConstructionScript`)