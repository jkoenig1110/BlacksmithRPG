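; CragNode is a harvestable ore node that gives the player a stack of copper, tin or iron ore.
; Overlap enables input, and each tick a short camera line trace, drawn for debug, checks whether the player is looking at the ore mesh.
; Interacting while aimed builds an ore item from the OreTable row, adds it to the inventory and destroys the node.
; CurrentMetal selects both that row and the construction-time mesh material.
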(event `self.ReceiveActorBeginOverlap`
  (params (OtherActor :type "Actor Object Reference"))
  (cast `/Game/Blueprints/Player/PlayerBP` OtherActor)
  (`self.EnableInput` (`GameplayStatics.GetPlayerController` 0))
  (set `self.PlayerNear` true))

(event `self.ReceiveActorEndOverlap`
  (params (OtherActor :type "Actor Object Reference"))
  (cast `/Game/Blueprints/Player/PlayerBP` OtherActor)
  (`self.DisableInput` (`GameplayStatics.GetPlayerController` 0))
  (set `self.PlayerNear` false))

(event `self.ReceiveTick`
  (params (DeltaSeconds :type "Float (single-precision)"))
  (if (`self.PlayerNear`)
    (bind _asplayer_bp (cast `/Game/Blueprints/Player/PlayerBP` (stale `self.ReceiveActorBeginOverlap` OtherActor)))
    (bind _camera (`/Game/Blueprints/Player/PlayerBP.Camera` _asplayer_bp))
    (bind _returnvalue (`SceneComponent.K2_GetComponentLocation` _camera))
    (bind _outhit (`KismetSystemLibrary.LineTraceSingle` :`Start` _returnvalue :`End` (+ _returnvalue (* (`SceneComponent.GetForwardVector` _camera) 150)) :`TraceChannel` "TraceTypeQuery1" :`DrawDebugType` "ForOneFrame" :`bIgnoreSelf` false))
    (if (== (`.HitComponent` (`GameplayStatics.BreakHitResult` _outhit)) (`self.Oremesh`))
      (set `self.PlayerIsLooking` true)
      (else
        (set `self.PlayerIsLooking` false)))))

(event `InputAction|Interact` :consume false
  (params (Key :type "Key Structure"))
  (:`Pressed`
    (if (and (`self.PlayerNear`) (`self.PlayerIsLooking`))
      (bind _returnvalue (`|GenericCreateObject` "/Game/Blueprints/Inventory/ItemObject/Item_Ore.Item_Ore_C" self null))
      (set `self.Ore Output` _returnvalue)
      (bind _returnvalue_2 (`|GetDataTableRow` "/Game/Blueprints/Inventory/Data/OreTable.OreTable" (`KismetStringLibrary.Conv_StringToName` (select `/Game/Blueprints/Inventory/Data/EMaterial` (`self.CurrentMetal`) :`NewEnumerator0` "Ore_Copper" :`NewEnumerator1` "Ore_Tin" :`NewEnumerator2` "Ore_Iron")))
        (:`then`
          (`/Game/Blueprints/Inventory/ItemObject/Item_Generic.Constructor` :`self` _returnvalue :`InOreStruct` _returnvalue_2)
          (`/Game/Blueprints/Inventory/ItemObject/Item_Generic.SetAmountInStack` (`self.Ore Output`) 5)
          (`/Game/Blueprints/Inventory/InventoryManager.AddItem` (`/Game/Blueprints/Player/ControllerBP.PlayerInventory` (cast `/Game/Blueprints/Player/ControllerBP` (`Pawn.GetController` (cast `/Game/Blueprints/Player/PlayerBP` (stale `self.ReceiveActorBeginOverlap` OtherActor) :!pure true)) :!pure true)) (`self.Ore Output`))
          (`self.K2_DestroyActor`))))))

(fn `UserConstructionScript`
  (`PrimitiveComponent.SetMaterial` (`self.Oremesh`) 0 (select `/Game/Blueprints/Inventory/Data/EMaterial` (`self.CurrentMetal`) :`NewEnumerator0` "/Game/Materials/Metals/MI_Cartoon_Copper_Instance.MI_Cartoon_Copper_Instance" :`NewEnumerator1` "/Game/Materials/Metals/MI_Cartoon_Tin_Instance.MI_Cartoon_Tin_Instance" :`NewEnumerator2` "/Game/Materials/Metals/MI_Cartoon_Iron_Instance.MI_Cartoon_Iron_Instance" :!type "MaterialInterface Object Reference")))