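; Inventory item for a metal ingot, holding its category, icon, mesh, stack data, metal and quality.
; Its Constructor event acts as a copy constructor when given a valid example item, reading each property through a cast to Item_Ingot.
; Without a valid example, it fills the same properties from the InIngotStruct data.
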(event `self.Constructor`
  (params (InExampleItem :type "/Game/Blueprints/Inventory/Item_Generic Object Reference") (InOreStruct :type "/Game/Blueprints/Inventory/Data/ItemStruct_Ore Structure") (InIngotStruct :type "/Game/Blueprints/Inventory/Data/ItemStruct_Ingot Structure"))
  (bind _asitem_ingot (cast `/Game/Blueprints/Inventory/Item_Ingot` InExampleItem :!pure true))
  (`/Engine/EditorBlueprintResources/StandardMacros.IsValid` InExampleItem
    (:`Is Valid`
      (set `self.Category` (`/Game/Blueprints/Inventory/Item_Generic.Category` _asitem_ingot))
      (set `self.Icon` (`/Game/Blueprints/Inventory/Item_Generic.Icon` _asitem_ingot))
      (set `self.BaseMesh` (`/Game/Blueprints/Inventory/Item_Generic.BaseMesh` _asitem_ingot))
      (set `self.MaxStack` (`/Game/Blueprints/Inventory/Item_Generic.MaxStack` _asitem_ingot))
      (set `self.AmountInStack` (`/Game/Blueprints/Inventory/Item_Generic.AmountInStack` _asitem_ingot))
      (set `self.IngotMetal` (`/Game/Blueprints/Inventory/Item_Ingot.IngotMetal` _asitem_ingot))
      (set `self.IngotQuality` (`/Game/Blueprints/Inventory/Item_Ingot.IngotQuality` _asitem_ingot)))
    (:`Is Not Valid`
      (set `self.Category` InIngotStruct_InItemCategory_5_E6CF8D9F423DB9D9C2F5229BEB1AB933)
      (set `self.Icon` InIngotStruct_InIcon_8_58D784C645086CAD15C260915C693843)
      (set `self.BaseMesh` InIngotStruct_InMesh_10_4732C377405C07C8AE52F9904B396652)
      (set `self.MaxStack` InIngotStruct_InMaxStack_13_7767E33F428548C52E14F88C95CF18DC)
      (set `self.AmountInStack` InIngotStruct_InAmountInStack_19_033292674CF398CA9AB6A7924EDDE4BD)
      (set `self.IngotMetal` InIngotStruct_InMetal_25_DA5C5B8B460F4CCF7991D286EC797577)
      (set `self.IngotQuality` InIngotStruct_InQuality_28_8E8FA8B140783B7A3C99F3973B208C22))))