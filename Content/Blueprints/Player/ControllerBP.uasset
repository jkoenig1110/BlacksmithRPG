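; Player controller that handles first-person-style look, movement and jump input for the controlled pawn and owns the player's inventory.
; On BeginPlay it constructs a 24-slot InventoryManager and passes it to PlayerHUD.
; E toggles the inventory widget along with cursor and input mode, calling the HUD's DropItemUI when closing.
; Q loops through the inventory array, dropping items by index.
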(event `self.ReceiveBeginPlay`
  (bind _returnvalue (`|GenericCreateObject` "/Game/Blueprints/Inventory/InventoryManager.InventoryManager_C" self (`self.K2_GetPawn`) (`self.GetHUD`)))
  (bind _output_get (set `self.PlayerInventory` _returnvalue))
  (`/Game/Blueprints/Inventory/InventoryManager.Constructor` _output_get 24)
  (`/Game/Blueprints/Player/PlayerHUD.SetInventory` (cast `/Game/Blueprints/Player/PlayerHUD` (`self.GetHUD`) :!pure true) _output_get))

(event `InputAxis|LookRight`
  (params (AxisValue :type "Float (single-precision)"))
  ;[1 1 1] Movement
  (`self.AddYawInput` AxisValue))

(event `InputAxis|LookUp`
  (params (AxisValue :type "Float (single-precision)"))
  ;[1 1 1] Movement
  (`self.AddPitchInput` AxisValue))

(event `InputAxis|MoveRight`
  (params (AxisValue :type "Float (single-precision)"))
  (bind _returnvalue (`self.K2_GetPawn`))
  ;[1 1 1] Movement
  (`Pawn.AddMovementInput` _returnvalue (`self.GetActorRightVector` _returnvalue) AxisValue false))

(event `InputAxis|MoveForward`
  (params (AxisValue :type "Float (single-precision)"))
  (bind _returnvalue (`self.K2_GetPawn`))
  ;[1 1 1] Movement
  (`Pawn.AddMovementInput` _returnvalue (`self.GetActorForwardVector` _returnvalue) AxisValue false))

(event `Key|E`
  (params (Key :type "Key Structure"))
  (bind _asplayer_hud (cast `/Game/Blueprints/Player/PlayerHUD` (`self.GetHUD`) :!pure true))
  (bind _playerinventoryui (`/Game/Blueprints/Player/PlayerHUD.PlayerInventoryUI` _asplayer_hud))
  (:`Pressed`
    (if (`Widget.IsInViewport` _playerinventoryui)
      (`/Game/Blueprints/Player/PlayerHUD.DropItemUI` _asplayer_hud)
      (`Widget.RemoveFromParent` _playerinventoryui)
      (`WidgetBlueprintLibrary.SetInputMode_GameOnly` self)
      (set `self.bShowMouseCursor` false)
      (else
        (`UserWidget.AddToViewport` _playerinventoryui 0)
        (`WidgetBlueprintLibrary.SetInputMode_GameAndUIEx` self (`/Game/Blueprints/Inventory/InventoryManager.AttachedUI` (`self.PlayerInventory`)) "LockAlways")
        (set `self.bShowMouseCursor` true)))))

(event `InputAction|Jump`
  (params (Key :type "Key Structure"))
  (bind _ascharacter (cast `Character` (`self.K2_GetPawn`) :!pure true))
  ;[1 1 1] Movement
  (:`Pressed`
    (`Character.Jump` _ascharacter))
  (:`Released`
    (`Character.StopJumping` _ascharacter)))

(event `Key|Q`
  (params (Key :type "Key Structure"))
  (:`Pressed`
    (for (_ _array_index) (`/Game/Blueprints/Inventory/InventoryManager.InventoryArray` (`self.PlayerInventory`))
      (`/Game/Blueprints/Inventory/InventoryManager.DropItemAtIndex` (`self.PlayerInventory`) _array_index))))

(fn `UserConstructionScript`)