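; GenericItemActor is a pickup item actor that carries inventory data and notifies the player on contact.
; On BeginPlay it builds an ItemData struct from its ID, name, max stack and the static mesh of its ItemMesh component.
; When a PlayerBP overlaps it, it passes itself to that player's SteppedOnItem, leaving the response to the player.
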(event `self.ReceiveBeginPlay`
  (set `self.ItemData` (make `/Game/Blueprints/Inventory/ItemDataStruct` (`self.ItemID`) (`self.ItemName`) (`StaticMeshComponent.StaticMesh` (`self.ItemMesh`)) (`self.MaxStack`))))

(event `self.ReceiveActorBeginOverlap`
  (params (OtherActor :type "Actor Object Reference"))
  (bind _asplayer_bp (cast `/Game/Blueprints/Player/PlayerBP` OtherActor))
  (`/Game/Blueprints/Player/PlayerBP.SteppedOnItem` _asplayer_bp self))

(fn `UserConstructionScript`)