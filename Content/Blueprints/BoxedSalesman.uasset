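; BoxedSalesman is an actor with a cat in a box that peeks out as the player approaches.
; Begin and end overlap with a PlayerBP toggle a proximity flag, which gates the Tick update.
; Each tick, the horizontal distance from the player's camera to the Centerpoint becomes an unclamped Lerp alpha that tilts the Lid open and raises the Cat as the player gets closer.
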(event `self.ReceiveTick`
  (params (DeltaSeconds :type "Float (single-precision)"))
  (bind (_returnvalue_x _returnvalue_y) (`KismetMathLibrary.BreakVector` (`SceneComponent.K2_GetComponentLocation` (`self.Centerpoint`))))
  (if (`self.PlayerClose`)
    (bind _asplayer_bp (cast `/Game/Blueprints/Player/PlayerBP` (stale `self.ReceiveActorBeginOverlap` OtherActor)))
    (bind (_returnvalue_x_2 _returnvalue_y_2) (`KismetMathLibrary.BreakVector` (`SceneComponent.K2_GetComponentLocation` (`/Game/Blueprints/Player/PlayerBP.Camera` _asplayer_bp))))
    (bind _output_get (set `self.PlayerDistance` (/ (`KismetMathLibrary.Sqrt` (+ (`KismetMathLibrary.Square` (- _returnvalue_x _returnvalue_x_2)) (`KismetMathLibrary.Square` (- _returnvalue_y _returnvalue_y_2)))) 480.0)))
    (`SceneComponent.K2_SetRelativeRotation` (`self.Lid`) (`KismetMathLibrary.RLerp` (struct :`Roll` 20.0) (struct) _output_get) false false)
    (`SceneComponent.K2_SetRelativeLocation` (`self.Cat`) (`KismetMathLibrary.MakeVector` 0.0 0.0 (`KismetMathLibrary.Lerp` 30.0 0.0 _output_get)) false false)))

(event `self.ReceiveActorBeginOverlap`
  (params (OtherActor :type "Actor Object Reference"))
  (cast `/Game/Blueprints/Player/PlayerBP` OtherActor)
  (set `self.PlayerClose` true))

(event `self.ReceiveActorEndOverlap`
  (params (OtherActor :type "Actor Object Reference"))
  (cast `/Game/Blueprints/Player/PlayerBP` OtherActor)
  (set `self.PlayerClose` false))

(fn `UserConstructionScript`)