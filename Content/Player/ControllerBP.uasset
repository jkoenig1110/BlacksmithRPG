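; Player controller Blueprint that turns look, move and jump input into actions on the controlled pawn.
; Look axes feed the controller's own yaw and pitch input, while move axes add movement along the pawn's right and forward vectors.
; Jump press and release cast the pawn to Character to start and stop jumping.
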(event `InputAxis|LookRight`
  (params (AxisValue :type "Float (single-precision)"))
  (`self.AddYawInput` AxisValue))

(event `InputAxis|LookUp`
  (params (AxisValue :type "Float (single-precision)"))
  (`self.AddPitchInput` AxisValue))

(event `InputAxis|MoveRight`
  (params (AxisValue :type "Float (single-precision)"))
  (bind _returnvalue (`self.K2_GetPawn`))
  (`Pawn.AddMovementInput` _returnvalue (`self.GetActorRightVector` _returnvalue) AxisValue false))

(event `InputAxis|MoveForward`
  (params (AxisValue :type "Float (single-precision)"))
  (bind _returnvalue (`self.K2_GetPawn`))
  (`Pawn.AddMovementInput` _returnvalue (`self.GetActorForwardVector` _returnvalue) AxisValue false))

(event `InputAction|Jump`
  (params (Key :type "Key Structure"))
  (bind _ascharacter (cast `Character` (`self.K2_GetPawn`) :!pure true))
  (:`Pressed`
    (`Character.Jump` _ascharacter))
  (:`Released`
    (`Character.StopJumping` _ascharacter)))

(fn `UserConstructionScript`)